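; Game mode Blueprint that shows the pause, level complete and level failed menus.
; The pause event creates its widget once and caches it, then adds or removes it from the viewport and toggles the mouse cursor.
; Level complete and failed events pause the game, create their widget, then share a path that shows the cursor and sets UI-only input.
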(event EventBeginPlay)

(event EventTick
  (params (DeltaSeconds :type Float%20%28single-precision%29)))

(event EventOnShowPauseMenu
  (params (_bShow :type Boolean))
  (bind _returnvalue (Game|GetPlayerController 0))
  (if _bShow
    (Utilities|IsValid (Variables|Default|GetRef_PauseMenu)
      (:Is%20Valid
        _)
      (:Is%20Not%20Valid
        (bind _returnvalue_2 (UserInterface|CreateWidget "/Game/PauseMenu/BP_WidgetPauseMenu.BP_WidgetPauseMenu_C"))
        (Variables|Default|SetRef_PauseMenu _returnvalue_2)))
    (UserInterface|Viewport|AddtoViewport (Variables|Default|GetRef_PauseMenu) 0)
    (Variables|/Script/Engine.PlayerController|SetbShowMouseCursor _returnvalue true)
    (else
      (Widget|RemovefromParent (Variables|Default|GetRef_PauseMenu))
      (Variables|/Script/Engine.PlayerController|SetbShowMouseCursor _returnvalue false))))

(event EventOnShowLevelCompleteMenu
  (bind _returnvalue (Game|GetPlayerController 0))
  (Game|SetGamePaused true)
  (bind _returnvalue_2 (UserInterface|CreateWidget "/Game/PauseMenu/BP_WidgetLevelComplete.BP_WidgetLevelComplete_C"))
  (UserInterface|Viewport|AddtoViewport _returnvalue_2 0)
  (Variables|/Script/Engine.PlayerController|SetbShowMouseCursor _returnvalue true)
  (Input|SetInputModeUIOnly _returnvalue 0 "DoNotLock"))

(event EventOnShowLevelFailedMenu
  (bind _returnvalue (Game|GetPlayerController 0))
  (Game|SetGamePaused true)
  (bind _returnvalue_2 (UserInterface|CreateWidget "/Game/PauseMenu/BP_WidgetLevelFailed.BP_WidgetLevelFailed_C"))
  (UserInterface|Viewport|AddtoViewport _returnvalue_2 0)
  (Variables|/Script/Engine.PlayerController|SetbShowMouseCursor _returnvalue true)
  (Input|SetInputModeUIOnly _returnvalue 0 "DoNotLock"))

(fn ConstructionScript)