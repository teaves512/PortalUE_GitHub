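; Temporary directional jump pad that flings the player character along the direction its Arrow component points.
; On Box overlap it zeroes the character's movement velocity, then launches it at a fixed speed along the Arrow's forward vector.
; Clearing velocity first keeps incoming momentum out of the launch, even though both override flags are off.
; An unconnected leftover launch with an explosion sound never runs.
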(event OnComponentBeginOverlap(Box)
  (params (OverlappedComponent :type Primitive%20Component%20Object%20Reference) (OtherActor :type Actor%20Object%20Reference) (OtherComp :type Primitive%20Component%20Object%20Reference) (OtherBodyIndex :type Integer) (bFromSweep :type Boolean) (SweepResult :type Hit%20Result%20Structure%20%28by%20ref%29))
  (bind _asplayer_character (Utilities|Casting|CastToPlayerCharacter OtherActor))
  (Variables|/Script/Engine.MovementComponent|SetVelocity (Variables|/Script/Engine.Character|GetCharacterMovement _asplayer_character) "0, 0, 0")
  (Character|LaunchCharacter _asplayer_character (* (Math|Vector|GetForwardVector (Variables|Default|GetArrow)) 2e+03) false false))

(event EventBeginPlay)

(event EventTick
  (params (DeltaSeconds :type Float%20%28single-precision%29)))

(fn ConstructionScript)